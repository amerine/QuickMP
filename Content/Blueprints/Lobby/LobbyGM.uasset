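; Lobby game mode that registers joining players, shares lobby state with them and launches the match.
; On login it reads server settings from the game instance, initializes the LobbyPC and possesses a base pawn at a random PlayerStart.
; It pushes player info, available characters and map settings to every LobbyPC, tracks start readiness from character picks, and server-travels by map ID.
; Character swapping and kick-list handling are empty stubs.
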(event Custom|SwapCharacter
  (params (PlayerController :type Player%20Controller%20Object%20Reference) (CharacterClass :type Character%20Class%20Reference) (ChangedStatus :type Boolean)))

(event Custom|EveryoneUpdate
  (bind _allplayercontrollers (Variables|ServerSettings|GetAllPlayerControllers))
  ;[1 1 1] Updates All COnncted players information when called
  (bind _output_get (Variables|ServerSettings|SetCurrentPlayers (Utilities|Array|Length (Variables|ServerSettings|GetAllPlayerControllers))))
  (if (> _output_get 0)
    (Utilities|Array|Clear (Variables|ServerSettings|GetConnectedPlayers))
    (for _array_element _allplayercontrollers
      (bind _aslobby_pc (Utilities|Casting|CastToLobbyPC _array_element))
      (Utilities|Array|Add (Variables|ServerSettings|GetConnectedPlayers) (Variables|/Game/Blueprints/Lobby/LobbyPC.LobbyPC_C|GetPlayerSettings _aslobby_pc))
      (Default|UpdateNumberOfPlayers _aslobby_pc (Variables|ServerSettings|GetCurrentPlayers) (Variables|ServerSettings|GetMaxPlayers)))
    (for _array_element_2 _allplayercontrollers
      (bind _aslobby_pc_2 (Utilities|Casting|CastToLobbyPC _array_element_2))
      (Default|AddPlayerInfo _aslobby_pc_2 (Variables|ServerSettings|GetConnectedPlayers))
      (Default|UpdateAvailableCharacters _aslobby_pc_2 (Variables|ServerSettings|GetAvailableCharacters))
      (CallFunction|AddtoKickList))
    (bind _array_element_3 (Utilities|Array|ForEachLoopwithBreak (Variables|ServerSettings|GetConnectedPlayers))
      (:LoopBody
        (if (== (.MyPlayerCharacter (Utilities|Struct|BreakPlayerInfo _array_element_3)) "/Game/Blueprints/Characters/0_Base.0_Base_C")
          (Variables|ServerSettings|SetCanWeStart? false)
          (CallFunction|CannotStartGame)
          (else
            (Variables|ServerSettings|SetCanWeStart? true)))))))

(event Custom|RespawnPlayer
  (params (PlayerController :type Player%20Controller%20Object%20Reference))
  (bind _returnvalue (Pawn|GetControlledPawn PlayerController))
  (bind _spawnpoints (Variables|ServerSettings|GetSpawnPoints))
  ;[1 1 1] Spawn Player as Base Character
  (Utilities|IsValid _returnvalue
    (:Is%20Valid
      (Actor|DestroyActor _returnvalue))
    (:Is%20Not%20Valid
      _))
  (bind _returnvalue_2 (Game|SpawnActorfromClass "/Game/Blueprints/Characters/0_Base.0_Base_C" (Transformation|GetActorTransform (Utilities|Array|Get(acopy) _spawnpoints (Math|Random|RandomIntegerinRange 0 (- (Utilities|Array|Length _spawnpoints) 1)))) "Undefined" 0 0))
  (Pawn|Possess PlayerController _returnvalue_2)
  (CallFunction|EveryoneUpdate))

(event Custom|LaunchTheGame
  (bind _returnvalue (Game|GetPlayerController 0))
  ;[1 1 1] Launch game based on map settings
  (switch int (Variables|ServerSettings|GetGM_MapID)
    (:0
      (Development|ExecuteConsoleCommand "servertravel /Game/Maps/Arena01" _returnvalue))
    (:1
      (Development|ExecuteConsoleCommand "servertravel /Game/Maps/Arena02" _returnvalue))))

(event Custom|AddToKickList
  ;[1 1 1] Updates All COnncted players information when called
)

(event Custom|CannotStartGame
  ;[1 1 1] Updates All COnncted players information when called
  (Utilities|Array|ForEachLoopwithBreak (Variables|ServerSettings|GetConnectedPlayers)) ; enters at Break
)

(event Custom|ServerUpdateGameSettings
  (params (MapImage :type Texture%202D%20Object%20Reference) (MapName :type Text) (MapTime :type Text) (MapID :type Integer))
  ;[1 1 1] Server has made changes update each client
  (Variables|ServerSettings|SetGM_MapImage MapImage)
  (Variables|ServerSettings|SetGM_MapTime MapName)
  (Variables|ServerSettings|SetGM_MapTime MapTime)
  (Variables|ServerSettings|SetGM_MapID MapID)
  (for _array_element (Variables|ServerSettings|GetAllPlayerControllers)
    (bind _aslobby_pc (Utilities|Casting|CastToLobbyPC _array_element))
    (Default|UpdateLobbySettings _aslobby_pc (Variables|ServerSettings|GetGM_MapImage) (Variables|ServerSettings|GetGM_MapName) (Variables|ServerSettings|GetGM_MapTime))))

(event EventPostLogin
  (params (NewPlayer :type Player%20Controller%20Object%20Reference))
  ;[1 1 1] Initial Setup
  (Networking|SwitchHasAuthority
    (:Authority
      (Utilities|Array|Add (Variables|ServerSettings|GetAllPlayerControllers) NewPlayer)
      (bind _outactors (Actor|GetAllActorsOfClass "/Script/Engine.PlayerStart"))
      (Variables|ServerSettings|SetSpawnPoints _outactors)
      (bind _asgame_info_instance (Utilities|Casting|CastToGameInfoInstance (Game|GetGameInstance)))
      (Variables|ServerSettings|SetServerName (Variables|/Game/Blueprints/All_Levels/GameInfoInstance.GameInfoInstance_C|GetServerName _asgame_info_instance))
      (Variables|ServerSettings|SetMaxPlayers (Variables|/Game/Blueprints/All_Levels/GameInfoInstance.GameInfoInstance_C|GetMaxPlayers _asgame_info_instance))
      (bind _aslobby_pc (Utilities|Casting|CastToLobbyPC NewPlayer))
      (Default|InitialSetup _aslobby_pc)
      (Default|SetupLobbyMenu _aslobby_pc (Variables|ServerSettings|GetServerName))
      (Default|UpdateLobbySettings _aslobby_pc (Variables|ServerSettings|GetGM_MapImage) (Variables|ServerSettings|GetGM_MapName) (Variables|ServerSettings|GetGM_MapTime))
      (CallFunction|RespawnPlayer NewPlayer))))

(fn ConstructionScript)